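; BP_CardPosition is a trigger actor that turns a card from the hand into a board actor in the duel.
; On BeginPlay it looks up BP_ActorDuel, retrying on a short delay until it is found.
; When its Box overlaps a BP_CardBoard, it spawns a BP_CardMaster at that actor's transform using the duel's referenced card UI info.
; It then removes that card from the hand and screen and calls CardPosition on the main HUD.
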(event OnComponentBeginOverlap(Box)
  (params (OverlappedComponent :type Primitive%20Component%20Object%20Reference) (OtherActor :type Actor%20Object%20Reference) (OtherComp :type Primitive%20Component%20Object%20Reference) (OtherBodyIndex :type Integer) (bFromSweep :type Boolean) (SweepResult :type Hit%20Result%20Structure%20%28by%20ref%29))
  (bind _ref_actor_duel (Variables|Default|GetRef%20Actor%20Duel))
  (bind _refcardui (Variables|/Game/CardInfo/BP_ActorDuel.BP_ActorDuel_C|GetRefCardUI _ref_actor_duel))
  (bind _cardcomponent (Variables|/Game/CardInfo/BP_ActorDuel.BP_ActorDuel_C|GetCardComponent _ref_actor_duel))
  (bind _asbp_card_board (Utilities|Casting|CastToBP_CardBoard OtherActor))
  (Game|SpawnActorfromClass "/Game/CardInfo/HUD/BP_CardMaster.BP_CardMaster_C" (Transformation|GetActorTransform _asbp_card_board) "Undefined" "MultiplyWithRoot" 0 (Variables|/Game/CardInfo/HUD/WB_CardUI.WB_CardUI_C|GetCardInfo (Variables|/Game/CardInfo/BP_ActorDuel.BP_ActorDuel_C|GetRefCardUI (Variables|Default|GetRef%20Actor%20Duel))) 0)
  (Utilities|Array|RemoveItem (Variables|/Game/CardInfo/CardComponent.CardComponent_C|Gethand _cardcomponent) _refcardui)
  (Widget|RemovefromParent _refcardui)
  (Default|CardPosition (Variables|/Game/CardInfo/CardComponent.CardComponent_C|GetRefMainHud _cardcomponent)))

(event EventBeginPlay
  (bind _returnvalue (Actor|GetActorOfClass "/Game/CardInfo/BP_ActorDuel.BP_ActorDuel_C" :!label _label))
  (Utilities|IsValid _returnvalue
    (:Is%20Valid
      (Variables|Default|SetRef%20Actor%20Duel _returnvalue))
    (:Is%20Not%20Valid
      (Utilities|FlowControl|Delay 0.2)
      (goto _label))))

(fn ConstructionScript)